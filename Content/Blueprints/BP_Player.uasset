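; Player actor for a shooter that moves along world X, fires projectiles and calls GameOver on BP_GameMode when health runs out.
; A spawn timeline raises and spins it, then sets MoveEnabled, which gates firing but not movement.
; Axis input eases horizontal speed, which Tick applies with sweep and turns into yaw tilt.
; Held fire retries on a looping timer, spawning only when its previous projectile is gone.
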(event Custom|PrimFire
  (CallFunction|PrimaryFire (Transformation|GetWorldTransform (Variables|Default|GetProjectileSpawn))))

(event EventBeginPlay
  ;[1 1 1] Player Spawn Animation
  (bind _asbp_game_mode (Utilities|Casting|CastToBP_GameMode (Game|GetGameMode)))
  (Variables|Default|SetBP_GameMode _asbp_game_mode)
  (Variables|Default|SetYaw (.Yaw (Math|Rotator|BreakRotator (Transformation|GetActorRotation))))
  (Variables|Default|SetSpawnLocation (Transformation|GetActorLocation))
  (bind _speed (Timeline|SpawnAnimation Play)
    (:Update
      (Transformation|SetActorLocation (Math|Vector|Lerp(Vector) (Variables|Default|GetSpawnLocation) (+ (Variables|Default|GetSpawnLocation) "0, 0,60.000000") _speed) false false)
      (Transformation|SetActorRotation (Math|Rotator|Lerp(Rotator) "0, 0, 0" (Math|Rotator|MakeRotator 0.0 0.0 (+ (Variables|Default|GetYaw) (* 3.6e+02 (Variables|Default|GetSpinCount)))) _speed)))
    (:Finished
      (Variables|Default|SetMoveEnabled true))))

(event EventTick
  (params (DeltaSeconds :type Float%20%28single-precision%29))
  ;[1 1 1] Movement
  (Variables|Default|SetDeltaSeconds DeltaSeconds)
  (Transformation|SetActorLocation (+ (Transformation|GetActorLocation) (Math|Vector|MakeVector (Variables|Default|GetHozSpeed) 0.0 (Variables|Default|GetVertSpeed))) true false)
  (Transformation|SetActorRotation (Class|KismetMathLibrary|RInterptoConstant (Transformation|GetActorRotation) (Math|Rotator|MakeRotator 0.0 0.0 (+ (* (Variables|Default|GetHozSpeed) -1e+01) (Variables|Default|GetYaw))) (Variables|Default|GetDeltaSeconds) 8e+01)))

(event Game|Damage|EventAnyDamage
  (params (Damage :type Float%20%28single-precision%29) (DamageType :type Damage%20Type%20Object%20Reference) (InstigatedBy :type Controller%20Object%20Reference) (DamageCauser :type Actor%20Object%20Reference))
  (Variables|Default|SetHealth (Math|Float|Clamp(Float) (- (Variables|Default|GetHealth) Damage) 0.0 (Variables|Default|GetMaxHealth)))
  (if (<= (Variables|Default|GetHealth) 0.0)
    (Default|GameOver (Variables|Default|GetBP_GameMode))
    (Actor|DestroyActor)))

(event Input|ActionEvents|InputActionPrimaryFire
  (params (Key :type Key%20Structure))
  (:Pressed
    (if (Variables|Default|GetMoveEnabled)
      (Utilities|Time|SetTimerbyFunctionName 0 "PrimFire" 0.2 true)
      (CallFunction|PrimaryFire (Transformation|GetWorldTransform (Variables|Default|GetProjectileSpawn)))))
  (:Released
    (Utilities|Time|ClearTimerbyFunctionName 0 "PrimFire")))

(event Input|AxisEvents|InputAxisMoveRight
  (params (AxisValue :type Float%20%28single-precision%29))
  ;[1 1 1] PlayerInput
  (bind _returndirectionspeed (CallFunction|Movement (Variables|Default|GetHozSpeed) AxisValue))
  (Variables|Default|SetHozSpeed _returndirectionspeed))

(fn ConstructionScript
  (Variables|Default|SetHealth (Variables|Default|GetMaxHealth)))

(fn Movement
  (params (Speed :type Float%20%28single-precision%29) (Direction :type Float%20%28single-precision%29))
  (return (Math|Interpolation|FInterpTo Speed (* Direction (Variables|Default|GetMovementSpeed)) (Variables|Default|GetDeltaSeconds) 6.0)))

(fn PrimaryFire
  (params (SpawnTransform :type Transform))
  (Utilities|IsValid (Variables|Default|GetOwnProjectile)
    (:Is%20Not%20Valid
      (Audio|PlaySoundatLocation "/Game/Assets/Audio/Shot.Shot" (Transformation|GetWorldLocation (Variables|Default|GetPlayerMesh)) "0, 0, 0" 1.0 1.0 0.0 0 0 0)
      (bind _returnvalue (Game|SpawnActorfromClass "/Game/Blueprints/BP_ProjectilePrimary.BP_ProjectilePrimary_C" SpawnTransform "AlwaysSpawn" 0 (LocalVariables|GetColour) self))
      (Variables|Default|SetOwnProjectile _returnvalue))))