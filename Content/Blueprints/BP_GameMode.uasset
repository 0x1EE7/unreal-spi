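; Game mode Blueprint that manages score, HUD and the game-over screen.
; On play it switches to game-only input, resets nothing but calls the score functions and shows BPW_HUD.
; SetScore adds to Score and raises TopScore when reached; LoadScore and SaveScore, called at begin and end of play, are empty stubs.
; GameOver shows BPW_GameOver, reveals the cursor and switches to UI-only input.
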(event EventBeginPlay
  (Input|SetInputModeGameOnly (Game|GetPlayerController 0))
  (CallFunction|LoadScore)
  (CallFunction|SetScore)
  (bind _returnvalue (UserInterface|CreateWidget "/Game/Blueprints/BPW_HUD.BPW_HUD_C"))
  (bind _output_get (Variables|Default|SetBPW_HUD _returnvalue))
  (UserInterface|Viewport|AddtoViewport _output_get 0))

(event EventTick
  (params (DeltaSeconds :type Float%20%28single-precision%29)))

(event EventEndPlay
  (params (EndPlayReason :type EEndPlayReason%20Enum :default "Destroyed"))
  (CallFunction|SaveScore))

(fn ConstructionScript)

(fn LoadScore)

(fn SaveScore)

(fn SetScore
  (params (Value :type Integer))
  (bind _output_get (Variables|Default|SetScore (+ Value (Variables|Default|GetScore))))
  (if (>= _output_get (Variables|Default|GetTopScore))
    (Variables|Default|SetTopScore (Variables|Default|GetScore))
    (else
      (Variables|Default|SetTopScore (Variables|Default|GetTopScore)))))

(fn GameOver
  (bind _returnvalue (Game|GetPlayerController 0))
  (bind _returnvalue_2 (UserInterface|CreateWidget "/Game/Blueprints/BPW_GameOver.BPW_GameOver_C"))
  (UserInterface|Viewport|AddtoViewport _returnvalue_2 0)
  (Variables|/Script/Engine.PlayerController|SetbShowMouseCursor _returnvalue true)
  (Input|SetInputModeUIOnly _returnvalue _returnvalue_2 "DoNotLock"))