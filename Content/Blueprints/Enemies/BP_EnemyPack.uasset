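; BP_EnemyPack is a spawner that lays out a grid formation of BP_EnemyOne actors when play begins.
; A loop from zero to MaxEnemies divides each index by MaxRows, using the quotient for the X step and the remainder for the Z step.
; Both steps scale by EnemySpacing and offset from the pack's location, so half-scale enemies fill the XZ plane and always spawn regardless of collision.
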(event EventBeginPlay
  (bind _enemyspacing (Variables|Default|GetEnemySpacing))
  (for _index (range 0 (Variables|Default|GetMaxEnemies))
    (Game|SpawnActorfromClass "/Game/Blueprints/Enemies/BP_EnemyOne.BP_EnemyOne_C" (Math|Transform|MakeTransform (+ (Transformation|GetActorLocation) (Math|Vector|MakeVector (* (Math|Conversions|ToFloat(Integer) (.ReturnValue (Math|Float|Division(WholeandRemainder) (Math|Conversions|ToFloat(Integer) _index) (Variables|Default|GetMaxRows)))) _enemyspacing) 0.0 (* _enemyspacing (.Remainder (Math|Float|Division(WholeandRemainder) (Math|Conversions|ToFloat(Integer) _index) (Variables|Default|GetMaxRows)))))) "0, 0, 0" "0.500000,0.500000,0.500000") "AlwaysSpawn" 0 0)))

(fn ConstructionScript)