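; BP_EnemyBase is a Space Invaders-style enemy that awards score and explodes audibly on any damage.
; A spawn timeline drops and spins it, then timers toggle stop-and-go movement and play a turning animation.
; All enemies share an X direction stored in BP_GameMode, flipped when one hits a side surface.
; While moving, it fires after random delays if the player passes an axis-weighted distance check, with at most two enemy projectiles alive.
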(event Custom|SleepMove
  (Variables|Default|SetMoveEnabled (not (Variables|Default|GetMoveEnabled))))

(event Custom|TurnEnemy
  (bind _shakevalue (Timeline|Timeline_0 PlayFromStart)
    (:Update
      (Transformation|SetActorRotation (Math|Rotator|Lerp(Rotator) "0, 0, 0" "0.000000,180.000000,0.000000" _shakevalue)))))

(event EventBeginPlay
  ;[1 1 1] Setup references and variables
  (bind _asbp_game_mode (Utilities|Casting|CastToBP_GameMode (Game|GetGameMode)))
  (bind _output_get (Variables|Default|SetBP_GameMode _asbp_game_mode))
  (Variables|/Game/Blueprints/BP_GameMode.BP_GameMode_C|SetMoveDirection _output_get false)
  (Variables|Default|SetSpawnLocation (Transformation|GetActorLocation))
  ;[1 1 1] SpawnAnimation
  (bind _entryspeed (Timeline|SpawnAnimation Play)
    (:Update
      (Transformation|SetActorLocationAndRotation (Math|Vector|Lerp(Vector) (Variables|Default|GetSpawnLocation) (- (Variables|Default|GetSpawnLocation) "0,0.000000,60.000000") _entryspeed) (Math|Rotator|Lerp(Rotator) "0, 0, 0" "0,360.000000, 0" _entryspeed) true)
      (Utilities|Time|SetTimerbyFunctionName 0 "SleepMove" 1.0 true)
      (Utilities|Time|SetTimerbyFunctionName 0 "TurnEnemy" 2.0 true))
    (:Finished
      (Variables|Default|SetMoveEnabled true))))

(event Game|Damage|EventAnyDamage
  (params (Damage :type Float%20%28single-precision%29) (DamageType :type Damage%20Type%20Object%20Reference) (InstigatedBy :type Controller%20Object%20Reference) (DamageCauser :type Actor%20Object%20Reference))
  (Default|SetScore (Variables|Default|GetBP_GameMode) 100)
  (Audio|PlaySoundatLocation "/Game/Assets/Audio/Explosion.Explosion" (Transformation|GetWorldLocation (Variables|Default|GetStaticMesh)) "0, 0, 0" 1.0 1.0 0.0 0 0 0)
  (Actor|DestroyActor))

(event EventTick
  (params (DeltaSeconds :type Float%20%28single-precision%29))
  ;[1 1 1] Movement
  (if (Variables|Default|GetMoveEnabled)
    (Transformation|SetActorLocation (+ (Transformation|GetActorLocation) (* (Math|Vector|MakeVector (* (Variables|Default|GetMoveSpeed) (Math|Float|SelectFloat 1.0 -1.0 (Variables|/Game/Blueprints/BP_GameMode.BP_GameMode_C|GetMoveDirection (Variables|Default|GetBP_GameMode)))) 0.0 0.0) DeltaSeconds)) true false)
    (Utilities|Fire)))

(event Collision|EventHit
  (params (MyComp :type Primitive%20Component%20Object%20Reference) (Other :type Actor%20Object%20Reference) (OtherComp :type Primitive%20Component%20Object%20Reference) (bSelfMoved :type Boolean) (HitLocation :type Vector :default "0, 0, 0") (HitNormal :type Vector :default "0, 0, 0") (NormalImpulse :type Vector :default "0, 0, 0") (Hit :type Hit%20Result%20Structure%20%28by%20ref%29))
  (bind _bp_gamemode (Variables|Default|GetBP_GameMode))
  ;[1 1 1] Movement
  (bind _output_get (Variables|Default|SetHitNormal HitNormal))
  (if (== 1.0 (Math|Float|Absolute(Float) (.x _output_get)))
    (Variables|/Game/Blueprints/BP_GameMode.BP_GameMode_C|SetMoveDirection _bp_gamemode (not (Variables|/Game/Blueprints/BP_GameMode.BP_GameMode_C|GetMoveDirection _bp_gamemode)))))

(fn ConstructionScript)